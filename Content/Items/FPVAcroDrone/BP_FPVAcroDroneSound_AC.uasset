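; Actor component that drives spatial motor audio for BP_FPVAcroDrone.
; On BeginPlay it attaches four propeller sounds at the thruster corners and a resting fan sound to the drone's root box.
; Each tick, every propeller's pitch and volume follow the strongest of throttle or its scaled-down, sign-split share of roll, yaw and pitch.
; The fan's volume runs inverse to throttle, fading out as power rises.
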(event EventBeginPlay
  (bind _returnvalue (Components|GetOwner))
  (bind _asbp_fpvacro_drone (Utilities|Casting|CastToBP_FPVAcroDrone _returnvalue)
    (:then
      (bind _asbox_collision (Utilities|Casting|CastToBoxComponent (Variables|/Script/Engine.Actor|GetRootComponent _returnvalue))
        (:then
          (bind _returnvalue_2 (Audio|SpawnSoundAttached "/FPVAcroDrones/Audio/A_Propeller_Cue.A_Propeller_Cue" _asbox_collision "None" (* (Math|Vector|MakeVector (Variables|/FPVAcroDrones/Items/FPVAcroDrone/BP_FPVAcroDrone.BP_FPVAcroDrone_C|GetThrusterDistance _asbp_fpvacro_drone) (Variables|/FPVAcroDrones/Items/FPVAcroDrone/BP_FPVAcroDrone.BP_FPVAcroDrone_C|GetThrusterDistance _asbp_fpvacro_drone) (Variables|/FPVAcroDrones/Items/FPVAcroDrone/BP_FPVAcroDrone.BP_FPVAcroDrone_C|GetThrusterOffset _asbp_fpvacro_drone)) "1.000000,1.000000,1.000000") "0, 0, 0" "KeepRelativeOffset" false 1.0 1.0 0.0 0 0))
          (bind _output_get (Variables|Default|SetAudioFrontRight _returnvalue_2))
          (Audio|Parameter|SetFloatParameter _output_get "Volume" 0.0 :!class /Script/AudioExtensions.AudioParameterControllerInterface)
          (bind _returnvalue_3 (Audio|SpawnSoundAttached "/FPVAcroDrones/Audio/A_Propeller_Cue.A_Propeller_Cue" _asbox_collision "None" (* (Math|Vector|MakeVector (Variables|/FPVAcroDrones/Items/FPVAcroDrone/BP_FPVAcroDrone.BP_FPVAcroDrone_C|GetThrusterDistance _asbp_fpvacro_drone) (Variables|/FPVAcroDrones/Items/FPVAcroDrone/BP_FPVAcroDrone.BP_FPVAcroDrone_C|GetThrusterDistance _asbp_fpvacro_drone) (Variables|/FPVAcroDrones/Items/FPVAcroDrone/BP_FPVAcroDrone.BP_FPVAcroDrone_C|GetThrusterOffset _asbp_fpvacro_drone)) "-1.000000,1.000000,1.000000") "0, 0, 0" "KeepRelativeOffset" false 1.0 1.0 0.0 0 0))
          (bind _output_get_2 (Variables|Default|SetAudioBackRight _returnvalue_3))
          (Audio|Parameter|SetFloatParameter _output_get_2 "Volume" 0.0 :!class /Script/AudioExtensions.AudioParameterControllerInterface)
          (bind _returnvalue_4 (Audio|SpawnSoundAttached "/FPVAcroDrones/Audio/A_Propeller_Cue.A_Propeller_Cue" _asbox_collision "None" (* (Math|Vector|MakeVector (Variables|/FPVAcroDrones/Items/FPVAcroDrone/BP_FPVAcroDrone.BP_FPVAcroDrone_C|GetThrusterDistance _asbp_fpvacro_drone) (Variables|/FPVAcroDrones/Items/FPVAcroDrone/BP_FPVAcroDrone.BP_FPVAcroDrone_C|GetThrusterDistance _asbp_fpvacro_drone) (Variables|/FPVAcroDrones/Items/FPVAcroDrone/BP_FPVAcroDrone.BP_FPVAcroDrone_C|GetThrusterOffset _asbp_fpvacro_drone)) "1.000000,-1.000000,1.000000") "0, 0, 0" "KeepRelativeOffset" false 1.0 1.0 0.0 0 0))
          (bind _output_get_3 (Variables|Default|SetAudioFrontLeft _returnvalue_4))
          (Audio|Parameter|SetFloatParameter _output_get_3 "Volume" 0.0 :!class /Script/AudioExtensions.AudioParameterControllerInterface)
          (bind _returnvalue_5 (Audio|SpawnSoundAttached "/FPVAcroDrones/Audio/A_Propeller_Cue.A_Propeller_Cue" _asbox_collision "None" (* (Math|Vector|MakeVector (Variables|/FPVAcroDrones/Items/FPVAcroDrone/BP_FPVAcroDrone.BP_FPVAcroDrone_C|GetThrusterDistance _asbp_fpvacro_drone) (Variables|/FPVAcroDrones/Items/FPVAcroDrone/BP_FPVAcroDrone.BP_FPVAcroDrone_C|GetThrusterDistance _asbp_fpvacro_drone) (Variables|/FPVAcroDrones/Items/FPVAcroDrone/BP_FPVAcroDrone.BP_FPVAcroDrone_C|GetThrusterOffset _asbp_fpvacro_drone)) "-1.000000,-1.000000,1.000000") "0, 0, 0" "KeepRelativeOffset" false 1.0 1.0 0.0 0 0))
          (bind _output_get_4 (Variables|Default|SetAudioBackLeft _returnvalue_5))
          (Audio|Parameter|SetFloatParameter _output_get_4 "Volume" 0.0 :!class /Script/AudioExtensions.AudioParameterControllerInterface)
          ;[0.15 0.15 0.15 0.5] Resting noise
          (bind _returnvalue_6 (Audio|SpawnSoundAttached "/FPVAcroDrones/Audio/A_Fan_Cue.A_Fan_Cue" _asbox_collision "None" "0, 0, 0" "0, 0, 0" "KeepRelativeOffset" false 1.0 1.0 0.0 0 0))
          (Audio|Parameter|SetFloatParameter _returnvalue_6 "Volume" (- 1.0 (Variables|/FPVAcroDrones/Items/FPVAcroDrone/BP_FPVAcroDrone.BP_FPVAcroDrone_C|GetThrottleCosmeticEffectStrength _asbp_fpvacro_drone)) :!class /Script/AudioExtensions.AudioParameterControllerInterface))
        (:CastFailed
          ;[1 0.1144 0.1356] Blueprint Assert
          (Class|BlueprintLoggingLibrary|LogFatal "Failed to get the root of BP_FPVAcroDrone"))))
    (:CastFailed
      (Class|BlueprintLoggingLibrary|LogFatal "Failed to cast to BP_FPVAcroDrone"))))

(event EventTick
  (params (DeltaSeconds :type Float%20%28single-precision%29))
  (CallFunction|SetPropellerSoundPower (Variables|Default|GetAudioFrontRight) (Math|Float|Max(Float) (Variables|/FPVAcroDrones/Items/FPVAcroDrone/BP_FPVAcroDrone.BP_FPVAcroDrone_C|GetThrottleCosmeticEffectStrength (stale EventBeginPlay _asbp_fpvacro_drone)) (* 0.1 (.PositiveSide (CallFunction|SplitPropellerPowerinTwoSides (Variables|/FPVAcroDrones/Items/FPVAcroDrone/BP_FPVAcroDrone.BP_FPVAcroDrone_C|GetRollCosmeticEffectStrength (stale EventBeginPlay _asbp_fpvacro_drone))))) (* 0.1 (.PositiveSide (CallFunction|SplitPropellerPowerinTwoSides (Variables|/FPVAcroDrones/Items/FPVAcroDrone/BP_FPVAcroDrone.BP_FPVAcroDrone_C|GetYawCosmeticEffectStrength (stale EventBeginPlay _asbp_fpvacro_drone))))) (* (.NegativeSide (CallFunction|SplitPropellerPowerinTwoSides (Variables|/FPVAcroDrones/Items/FPVAcroDrone/BP_FPVAcroDrone.BP_FPVAcroDrone_C|GetPitchCosmeticEffectStrength (stale EventBeginPlay _asbp_fpvacro_drone)))) 0.1)))
  (CallFunction|SetPropellerSoundPower (Variables|Default|GetAudioBackRight) (Math|Float|Max(Float) (Variables|/FPVAcroDrones/Items/FPVAcroDrone/BP_FPVAcroDrone.BP_FPVAcroDrone_C|GetThrottleCosmeticEffectStrength (stale EventBeginPlay _asbp_fpvacro_drone)) (* 0.1 (.PositiveSide (CallFunction|SplitPropellerPowerinTwoSides (Variables|/FPVAcroDrones/Items/FPVAcroDrone/BP_FPVAcroDrone.BP_FPVAcroDrone_C|GetRollCosmeticEffectStrength (stale EventBeginPlay _asbp_fpvacro_drone))))) (* (.NegativeSide (CallFunction|SplitPropellerPowerinTwoSides (Variables|/FPVAcroDrones/Items/FPVAcroDrone/BP_FPVAcroDrone.BP_FPVAcroDrone_C|GetYawCosmeticEffectStrength (stale EventBeginPlay _asbp_fpvacro_drone)))) 0.1) (* (.NegativeSide (CallFunction|SplitPropellerPowerinTwoSides (Variables|/FPVAcroDrones/Items/FPVAcroDrone/BP_FPVAcroDrone.BP_FPVAcroDrone_C|GetPitchCosmeticEffectStrength (stale EventBeginPlay _asbp_fpvacro_drone)))) 0.1)))
  (CallFunction|SetPropellerSoundPower (Variables|Default|GetAudioFrontLeft) (Math|Float|Max(Float) (Variables|/FPVAcroDrones/Items/FPVAcroDrone/BP_FPVAcroDrone.BP_FPVAcroDrone_C|GetThrottleCosmeticEffectStrength (stale EventBeginPlay _asbp_fpvacro_drone)) (* (.NegativeSide (CallFunction|SplitPropellerPowerinTwoSides (Variables|/FPVAcroDrones/Items/FPVAcroDrone/BP_FPVAcroDrone.BP_FPVAcroDrone_C|GetRollCosmeticEffectStrength (stale EventBeginPlay _asbp_fpvacro_drone)))) 0.1) (* (.NegativeSide (CallFunction|SplitPropellerPowerinTwoSides (Variables|/FPVAcroDrones/Items/FPVAcroDrone/BP_FPVAcroDrone.BP_FPVAcroDrone_C|GetYawCosmeticEffectStrength (stale EventBeginPlay _asbp_fpvacro_drone)))) 0.1) (* 0.1 (.PositiveSide (CallFunction|SplitPropellerPowerinTwoSides (Variables|/FPVAcroDrones/Items/FPVAcroDrone/BP_FPVAcroDrone.BP_FPVAcroDrone_C|GetPitchCosmeticEffectStrength (stale EventBeginPlay _asbp_fpvacro_drone)))))))
  (CallFunction|SetPropellerSoundPower (Variables|Default|GetAudioBackLeft) (Math|Float|Max(Float) (Variables|/FPVAcroDrones/Items/FPVAcroDrone/BP_FPVAcroDrone.BP_FPVAcroDrone_C|GetThrottleCosmeticEffectStrength (stale EventBeginPlay _asbp_fpvacro_drone)) (* (.NegativeSide (CallFunction|SplitPropellerPowerinTwoSides (Variables|/FPVAcroDrones/Items/FPVAcroDrone/BP_FPVAcroDrone.BP_FPVAcroDrone_C|GetRollCosmeticEffectStrength (stale EventBeginPlay _asbp_fpvacro_drone)))) 0.1) (* 0.1 (.PositiveSide (CallFunction|SplitPropellerPowerinTwoSides (Variables|/FPVAcroDrones/Items/FPVAcroDrone/BP_FPVAcroDrone.BP_FPVAcroDrone_C|GetYawCosmeticEffectStrength (stale EventBeginPlay _asbp_fpvacro_drone))))) (* 0.1 (.PositiveSide (CallFunction|SplitPropellerPowerinTwoSides (Variables|/FPVAcroDrones/Items/FPVAcroDrone/BP_FPVAcroDrone.BP_FPVAcroDrone_C|GetPitchCosmeticEffectStrength (stale EventBeginPlay _asbp_fpvacro_drone)))))))
  ;[0.15 0.15 0.15 0.5] Resting noise
  (Audio|Parameter|SetFloatParameter (stale EventBeginPlay _returnvalue_6) "Volume" (- 1.0 (Variables|/FPVAcroDrones/Items/FPVAcroDrone/BP_FPVAcroDrone.BP_FPVAcroDrone_C|GetThrottleCosmeticEffectStrength (stale EventBeginPlay _asbp_fpvacro_drone))) :!class /Script/AudioExtensions.AudioParameterControllerInterface))

(fn SetPropellerSoundPower
  (params (AudioComponent :type Audio%20Parameter%20Controller%20Interface%20Interface) (Power :type Float%20%28double-precision%29))
  (Audio|Parameter|SetFloatParameter AudioComponent "Pitch" Power :!class /Script/AudioExtensions.AudioParameterControllerInterface)
  (Audio|Parameter|SetFloatParameter AudioComponent "Volume" Power :!class /Script/AudioExtensions.AudioParameterControllerInterface))

(fn SplitPropellerPowerinTwoSides
  (params (Input :type Float%20%28double-precision%29))
  (return (* (Math|Float|Clamp(Float) Input -1.0 0.0) -1.0) (Math|Float|Clamp(Float) Input)))