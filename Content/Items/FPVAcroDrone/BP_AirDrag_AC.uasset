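; BP_AirDrag_AC is a component that applies air drag to its owning actor, part of the FPV acro drone item.
; On BeginPlay it caches the owner's root as a BoxComponent, logging a fatal error if the cast fails.
; Each tick, when that box's linear velocity exceeds a threshold, it adds a force opposite to the velocity, scaled by a drag coefficient and the square of speed.
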(event EventBeginPlay
  (bind _asbox_collision (Utilities|Casting|CastToBoxComponent (Variables|/Script/Engine.Actor|GetRootComponent (Components|GetOwner)))
    (:CastFailed
      ;[1 0.1144 0.1356] Blueprint Assert
      (Class|BlueprintLoggingLibrary|LogFatal "Failed to cast Root to BoxComponent"))))

(event EventTick
  (params (DeltaSeconds :type Float%20%28single-precision%29))
  (bind _returnvalue (Physics|GetPhysicsLinearVelocity (stale EventBeginPlay _asbox_collision) "None"))
  (if (> (Math|Vector|VectorLength _returnvalue) (Variables|Default|GetVelocityThreshold))
    (Physics|AddForce (stale EventBeginPlay _asbox_collision) (* -1.0 (Variables|Default|GetDragCoefficient) _returnvalue (Math|Vector|VectorLength _returnvalue)) "None" false)))