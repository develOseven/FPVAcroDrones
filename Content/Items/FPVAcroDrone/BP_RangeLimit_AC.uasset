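; Range-limit component that keeps an FPV acro drone near the pawn of its controlling player.
; Each tick it compares squared distance to that pawn, applying velocity-squared drag on the drone's box root past a near radius when speed exceeds a threshold.
; Past the outer limit it adds a distance-scaled pull-back force and logs it, though slow drones beyond the near radius skip this check.
; Failed owner or root casts log fatal errors.
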(event EventTick
  (params (DeltaSeconds :type Float%20%28single-precision%29))
  (bind _returnvalue (Components|GetOwner))
  (bind _returnvalue_2 (Transformation|GetActorLocation _returnvalue))
  (bind _asbp_fpvacro_drone (Utilities|Casting|CastToBP_FPVAcroDrone _returnvalue)
    (:then
      (bind _asbox_collision (Utilities|Casting|CastToBoxComponent (Variables|/Script/Engine.Actor|GetRootComponent _returnvalue))
        (:then
          (Utilities|IsValid (Variables|/FPVAcroDrones/Items/FPVAcroDrone/BP_FPVAcroDrone.BP_FPVAcroDrone_C|GetControlledBy _asbp_fpvacro_drone)
            (:Is%20Valid
              (if (> (Class|KismetMathLibrary|VectorDistanceSquared (Transformation|GetActorLocation (Pawn|GetControlledPawn (Variables|/FPVAcroDrones/Items/FPVAcroDrone/BP_FPVAcroDrone.BP_FPVAcroDrone_C|GetControlledBy _asbp_fpvacro_drone))) _returnvalue_2) (Variables|Default|GetNearLimitingRadiusSquared))
                ;[0.15 0.15 0.15 0.5] Drag
                (bind _returnvalue_3 (Physics|GetPhysicsLinearVelocity _asbox_collision "None"))
                (if (> (Math|Vector|VectorLength _returnvalue_3) (Variables|Default|GetVelocityThreshold))
                  (Physics|AddForce _asbox_collision (* -1.0 (Variables|Default|GetDragCoefficient) _returnvalue_3 (Math|Vector|VectorLength _returnvalue_3)) "None" false)
                  (if (> (Class|KismetMathLibrary|VectorDistanceSquared (Transformation|GetActorLocation (Pawn|GetControlledPawn (Variables|/FPVAcroDrones/Items/FPVAcroDrone/BP_FPVAcroDrone.BP_FPVAcroDrone_C|GetControlledBy _asbp_fpvacro_drone))) _returnvalue_2) (Variables|Default|GetLimitingRadiusSquared)) :!label _label
                    ;[0.15 0.15 0.15 0.5] Bounce
                    (Physics|AddForce _asbox_collision (* (- (Transformation|GetActorLocation (Pawn|GetControlledPawn (Variables|/FPVAcroDrones/Items/FPVAcroDrone/BP_FPVAcroDrone.BP_FPVAcroDrone_C|GetControlledBy _asbp_fpvacro_drone))) _returnvalue_2) (Variables|Default|GetForceMultiplier)) "None" false)
                    (Class|BlueprintLoggingLibrary|LogDisplay (Utilities|String|Append "Out of range: " (Utilities|String|ToString(Float) (Class|KismetMathLibrary|VectorDistanceSquared (Transformation|GetActorLocation (Pawn|GetControlledPawn (Variables|/FPVAcroDrones/Items/FPVAcroDrone/BP_FPVAcroDrone.BP_FPVAcroDrone_C|GetControlledBy _asbp_fpvacro_drone))) _returnvalue_2))))))
                (else
                  (goto _label))))))
        (:CastFailed
          ;[1 0.1144 0.1356] Blueprint Assert
          (Class|BlueprintLoggingLibrary|LogFatal "Failed to get the root of BP_FPVAcroDrone"))))
    (:CastFailed
      (Class|BlueprintLoggingLibrary|LogFatal "Failed to cast to BP_FPVAcroDrone"))))