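; Player-controlled FPV quadcopter drone that flies in acro style, with stick input driving local rotation rates.
; Throttle applies upward force to the physics body on Tick, at four local thruster points or centrally when thruster distance is zero, capping speed while throttling.
; Pitch, yaw and roll pass through an expo-style response curve, accumulating into a per-frame rotation.
; RPC events forward throttle, rotation and cosmetic effect strengths.
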(event Custom|Add%20Actor%20Local%20Rotation%20RPC
  (params (Delta%20Rorarion :type Rotator))
  (Transformation|AddActorLocalRotation Delta%20Rorarion false false))

(event Custom|Set%20YawCosmeticEffectStrength%20RPC
  (params (YawCosmeticEffectStrength :type Float%20%28double-precision%29))
  (Variables|Default|SetYawCosmeticEffectStrength YawCosmeticEffectStrength))

(event Custom|Set%20RollCosmeticEffectStrength%20RPC
  (params (RollCosmeticEffectStrength :type Float%20%28double-precision%29))
  (Variables|Default|SetRollCosmeticEffectStrength RollCosmeticEffectStrength))

(event Custom|Set%20Throttle%20Input%20RPC
  (params (Throttle%20Input :type Float%20%28double-precision%29))
  (Variables|Default|SetThrottleInput Throttle%20Input))

(event Custom|Set%20PitchCosmeticEffectStrength%20RPC
  (params (PitchCosmeticEffectStrength :type Float%20%28double-precision%29))
  (Variables|Default|SetPitchCosmeticEffectStrength PitchCosmeticEffectStrength))

(event Custom|Set%20ThrottleCosmeticEffectStrength%20RPC
  (params (ThrottleCosmeticEffectStrength :type Float%20%28double-precision%29))
  (Variables|Default|SetThrottleCosmeticEffectStrength ThrottleCosmeticEffectStrength))

(event Input|EnhancedActionEvents|EnhancedInputActionIA_Throttle
  (params (ActionValue :type Float%20%28double-precision%29) (ElapsedSeconds :type Float%20%28double-precision%29) (TriggeredSeconds :type Float%20%28double-precision%29) (InputAction :type Input%20Action%20Object%20Reference :default "/FPVAcroDrones/Input/Actions/IA_Throttle.IA_Throttle"))
  (:Triggered
    (if false
      (Variables|Default|SetThrottleCosmeticEffectStrength 0.0 :!label _label)
      (else
        (Variables|Default|SetThrottleCosmeticEffectStrength (Math|Float|Clamp(Float) ActionValue))))
    (CallFunction|SetThrottleCosmeticEffectStrengthRPC (Variables|Default|GetThrottleCosmeticEffectStrength))
    (CallFunction|SetThrottleInputRPC (Variables|Default|GetThrottleCosmeticEffectStrength)))
  (:Completed
    (goto _label)))

(event Input|EnhancedActionEvents|EnhancedInputActionIA_Pitch
  (params (ActionValue :type Float%20%28double-precision%29) (ElapsedSeconds :type Float%20%28double-precision%29) (TriggeredSeconds :type Float%20%28double-precision%29) (InputAction :type Input%20Action%20Object%20Reference :default "/FPVAcroDrones/Input/Actions/IA_Pitch.IA_Pitch"))
  (bind _output (CallFunction|ResponseCurve ActionValue))
  (bind _output_get (Variables|Default|SetPitchCosmeticEffectStrength ActionValue))
  (CallFunction|SetPitchCosmeticEffectStrengthRPC _output_get)
  (Class|BlueprintLoggingLibrary|LogDisplay (Utilities|String|Append "Pitch" (Utilities|String|ToString(Float) ActionValue)))
  (if (!= _output 0.0)
    (if (not false)
      (Variables|Default|SetRelativeInput (Math|Rotator|MakeRotator (.roll (Variables|Default|GetRelativeInput)) (+ _output (.pitch (Variables|Default|GetRelativeInput))) (.yaw (Variables|Default|GetRelativeInput))))
      (Variables|Default|SetHasRelativeRotation true))))

(event Input|EnhancedActionEvents|EnhancedInputActionIA_Yaw
  (params (ActionValue :type Float%20%28double-precision%29) (ElapsedSeconds :type Float%20%28double-precision%29) (TriggeredSeconds :type Float%20%28double-precision%29) (InputAction :type Input%20Action%20Object%20Reference :default "/FPVAcroDrones/Input/Actions/IA_Yaw.IA_Yaw"))
  (bind _output (CallFunction|ResponseCurve ActionValue))
  (bind _output_get (Variables|Default|SetYawCosmeticEffectStrength ActionValue))
  (CallFunction|SetYawCosmeticEffectStrengthRPC _output_get)
  (Class|BlueprintLoggingLibrary|LogDisplay (Utilities|String|Append "Yaw" (Utilities|String|ToString(Float) ActionValue)))
  (if (!= _output 0.0)
    (if (not false)
      (Variables|Default|SetRelativeInput (Math|Rotator|MakeRotator (.roll (Variables|Default|GetRelativeInput)) (.pitch (Variables|Default|GetRelativeInput)) (+ (.yaw (Variables|Default|GetRelativeInput)) _output)))
      (Variables|Default|SetHasRelativeRotation true))))

(event Input|EnhancedActionEvents|EnhancedInputActionIA_Roll
  (params (ActionValue :type Float%20%28double-precision%29) (ElapsedSeconds :type Float%20%28double-precision%29) (TriggeredSeconds :type Float%20%28double-precision%29) (InputAction :type Input%20Action%20Object%20Reference :default "/FPVAcroDrones/Input/Actions/IA_Roll.IA_Roll"))
  (bind _output (CallFunction|ResponseCurve ActionValue))
  (bind _output_get (Variables|Default|SetRollCosmeticEffectStrength ActionValue))
  (CallFunction|SetRollCosmeticEffectStrengthRPC _output_get)
  (Class|BlueprintLoggingLibrary|LogDisplay (Utilities|String|Append "Roll" (Utilities|String|ToString(Float) ActionValue)))
  (if (!= _output 0.0)
    (if (not false)
      (Variables|Default|SetRelativeInput (Math|Rotator|MakeRotator (+ (.roll (Variables|Default|GetRelativeInput)) _output) (.pitch (Variables|Default|GetRelativeInput)) (.yaw (Variables|Default|GetRelativeInput))))
      (Variables|Default|SetHasRelativeRotation true))))

(event EventTick
  (params (DeltaSeconds :type Float%20%28single-precision%29))
  (bind _throttleinput (Variables|Default|GetThrottleInput))
  (bind _thrusterforce (Variables|Default|GetThrusterForce))
  (bind _thrusteroffset (Variables|Default|GetThrusterOffset))
  (bind _thrusterdistance (Variables|Default|GetThrusterDistance))
  (bind _returnvalue (Math|Vector|MakeVector _thrusterdistance _thrusterdistance _thrusteroffset))
  (bind _returnvalue_2 (* _throttleinput _thrusterforce))
  (bind _returnvalue_3 (Math|Vector|MakeVector 0.0 0.0 _returnvalue_2))
  (Utilities|FlowControl|Sequence
    (:then_0
      (if (> (Variables|Default|GetThrottleInput) 0.0)
        (if (== (Variables|Default|GetThrusterDistance) 0.0)
          (Physics|AddForce (Variables|Default|GetQuadcopterCollision) (* _returnvalue_3 "4.000000,4.000000,4.000000") "None" false)
          (else
            (Class|PrimitiveComponent|AddForceatLocationLocal (Variables|Default|GetQuadcopterCollision) _returnvalue_3 (* _returnvalue "1.000000,1.000000,1.000000") "None")
            (Class|PrimitiveComponent|AddForceatLocationLocal (Variables|Default|GetQuadcopterCollision) _returnvalue_3 (* _returnvalue "-1.000000,1.000000,1.000000") "None")
            (Class|PrimitiveComponent|AddForceatLocationLocal (Variables|Default|GetQuadcopterCollision) _returnvalue_3 (* _returnvalue "1.000000,-1.000000,1.000000") "None")
            (Class|PrimitiveComponent|AddForceatLocationLocal (Variables|Default|GetQuadcopterCollision) _returnvalue_3 (* _returnvalue "-1.000000,-1.000000,1.000000") "None")))
        (bind _returnvalue_4 (Physics|GetPhysicsLinearVelocity (Variables|Default|GetQuadcopterCollision) "None"))
        (if (> (Math|Vector|VectorLength _returnvalue_4) (Variables|Default|GetMaxSpeed))
          (Physics|SetPhysicsLinearVelocity (Variables|Default|GetQuadcopterCollision) (* (Math|Vector|Normalize _returnvalue_4) (Variables|Default|GetMaxSpeed)) false "None"))))
    (:then_1
      (if (Variables|Default|GetHasRelativeRotation)
        (CallFunction|AddActorLocalRotationRPC (* (Variables|Default|GetRelativeInput) DeltaSeconds))
        (Variables|Default|SetRelativeInput "0, 0, 0")
        (Variables|Default|SetHasRelativeRotation false)))))

(fn ConstructionScript)

(fn ResponseCurve
  (params (Input :type Float%20%28double-precision%29))
  (return (* (Variables|Default|GetSpeed) Input (Math|Float|Lerp 1.0 (Math|Float|Power (Math|Float|Absolute(Float) Input) (* 2e+01 (Variables|Default|GetTransition))) (Variables|Default|GetPrecision)))))