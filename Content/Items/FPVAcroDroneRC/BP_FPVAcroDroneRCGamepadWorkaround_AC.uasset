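; Actor component on the FPV acro drone RC equipment that works around gamepad stick input for flying the drone.
; It gets the player controller from the owning equipment's callback and binds to raw analog events forwarded by the FPVAcroDrones world module.
; Each stick axis is injected into Enhanced Input as yaw, throttle, roll or pitch, with right stick Y inverted to correct Unreal's flipped axis.
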(event Custom|Event%20Was%20Equipped
  (params (PlayerController :type Player%20Controller%20Object%20Reference))
  ;[0.15 0.15 0.15 0.5] Get Player Controller from the Owning Actor
  (Variables|Default|SetPlayerController PlayerController))

(event Custom|On%20Controller%20Analog
  (params (Key%20Name :type Name) (Platform%20User%20Id :type Platform%20User%20Id%20Structure) (Input%20Device%20Id :type Input%20Device%20Id%20Structure) (Analog%20Value :type Float%20%28double-precision%29))
  (bind _playercontroller (Variables|Default|GetPlayerController))
  (bind _returnvalue (PlayerController|LocalPlayerSubsystems|GetEnhancedInputLocalPlayerSubsystem _playercontroller))
  (Utilities|IsValid (Variables|Default|GetPlayerController)
    (:Is%20Valid
      (switch name Key%20Name
        (:Gamepad_LeftX
          (Class|EnhancedInputSubsystemInterface|InjectInputVectorforAction _returnvalue "/FPVAcroDrones/Input/Actions/IA_Yaw.IA_Yaw" (Math|Vector|MakeVector Analog%20Value 0.0 0.0)))
        (:Gamepad_LeftY
          (Class|EnhancedInputSubsystemInterface|InjectInputVectorforAction _returnvalue "/FPVAcroDrones/Input/Actions/IA_Throttle.IA_Throttle" (Math|Vector|MakeVector Analog%20Value 0.0 0.0)))
        (:Gamepad_RightX
          (Class|EnhancedInputSubsystemInterface|InjectInputVectorforAction _returnvalue "/FPVAcroDrones/Input/Actions/IA_Roll.IA_Roll" (Math|Vector|MakeVector Analog%20Value 0.0 0.0)))
        (:Gamepad_RightY
          (Class|EnhancedInputSubsystemInterface|InjectInputVectorforAction _returnvalue "/FPVAcroDrones/Input/Actions/IA_Pitch.IA_Pitch" (Math|Vector|MakeVector (* Analog%20Value -1.0) 0.0 0.0)))))))

(event EventBeginPlay
  (Utilities|FlowControl|Sequence
    (:then_0
      ;[0.15 0.15 0.15 0.5] Get Player Controller from the Owning Actor
      (bind _asequip_fpvacro_drone_rc (Utilities|Casting|CastToEquip_FPVAcroDroneRC (Components|GetOwner))
        (:then
          (EventDispatchers|BindEventtoPlayerControllerSet _asequip_fpvacro_drone_rc (delegate Custom|Event%20Was%20Equipped)))
        (:CastFailed
          ;;[1 0.15 0.15 0.5] Blueprint Assert
          (Class|BlueprintLoggingLibrary|LogFatal "Can't get RC. Will not control the drone."))))
    (:then_1
      ;[0.15 0.15 0.15 0.5] Get Direct Gamepad Input
      (bind _asroot_game_world_fpvacro_drones (Utilities|Casting|CastToRootGameWorld_FPVAcroDrones (Class|WorldModuleManager|FindModule (Subsystems|GetWorldModuleManager) (Utilities|Name|MakeLiteralName "FPVAcroDrones")))
        (:then
          (EventDispatchers|BindEventtoForwardonControllerAnalog _asroot_game_world_fpvacro_drones (delegate Custom|On%20Controller%20Analog)))
        (:CastFailed
          ;;[1 0.15 0.15 0.5] Blueprint Assert
          (Class|BlueprintLoggingLibrary|LogFatal "Can't get RootGameWorld_FPVActoDrones."))))))