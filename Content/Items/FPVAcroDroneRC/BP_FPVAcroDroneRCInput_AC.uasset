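; Input component for the FPV acro drone remote control, merging gamepad and keyboard controls once its owning equipment supplies a player controller.
; Stick axes and key states, including a throttle trim ramped on Tick, are injected into intermediate actions, then forwarded to drone actions with response curves.
; Gates arbitrate devices: stick input blocks keyboard injection and resets the trim, while keyboard throttle keys reopen all four axes.
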(event Custom|Event%20Was%20Equipped
  (params (PlayerController :type Player%20Controller%20Object%20Reference))
  ;[0.15 0.15 0.15 0.5] Get Player Controller from the Owning Actor
  (Variables|Default|SetPlayerController PlayerController))

(event Input|EnhancedActionEvents|EnhancedInputActionIA_ThrottleUp
  (params (ActionValue :type Boolean) (ElapsedSeconds :type Float%20%28double-precision%29) (TriggeredSeconds :type Float%20%28double-precision%29) (InputAction :type Input%20Action%20Object%20Reference :default "/FPVAcroDrones/Input/Actions/IA_ThrottleUp.IA_ThrottleUp"))
  (bind _playercontroller (Variables|Default|GetPlayerController))
  (bind _returnvalue (PlayerController|LocalPlayerSubsystems|GetEnhancedInputLocalPlayerSubsystem _playercontroller))
  (:Triggered
    ;[0.15 0.15 0.15 0.5] Keyboard
    (Utilities|FlowControl|Sequence
      (:then_0
        ;;[0.15 0.15 0.15 0.5] Keyboard Throttle
        (bind _output_get (Variables|Default|SetGetIA_ThrottleUp true)))
      (:then_1
        ;;[0.15 0.15 0.15 0.5] Block Keyboard Input (note that Steam also adds arrow key events to the gamepad)
        (Utilities|FlowControl|Sequence
          (:then_0
            (Utilities|FlowControl|Gate false) ; enters at Open
          )
          (:then_1
            (Utilities|FlowControl|Gate false) ; enters at Open
          )
          (:then_2
            (Utilities|FlowControl|Gate false) ; enters at Open
          )
          (:then_3
            (Utilities|FlowControl|Gate false) ; enters at Open
          )))))
  (:Completed
    (Variables|Default|SetGetIA_ThrottleUp false)))

(event Input|EnhancedActionEvents|EnhancedInputActionIA_ThrottleDown
  (params (ActionValue :type Boolean) (ElapsedSeconds :type Float%20%28double-precision%29) (TriggeredSeconds :type Float%20%28double-precision%29) (InputAction :type Input%20Action%20Object%20Reference :default "/FPVAcroDrones/Input/Actions/IA_ThrottleDown.IA_ThrottleDown"))
  (bind _playercontroller (Variables|Default|GetPlayerController))
  (bind _returnvalue (PlayerController|LocalPlayerSubsystems|GetEnhancedInputLocalPlayerSubsystem _playercontroller))
  (:Triggered
    ;[0.15 0.15 0.15 0.5] Keyboard
    (Utilities|FlowControl|Sequence
      (:then_0
        ;;[0.15 0.15 0.15 0.5] Keyboard Throttle
        (Variables|Default|SetGetIA_ThrottleDown true))
      (:then_1
        ;;[0.15 0.15 0.15 0.5] Block Keyboard Input (note that Steam also adds arrow key events to the gamepad)
        (Utilities|FlowControl|Sequence
          (:then_0
            (Utilities|FlowControl|Gate false) ; enters at Open
          )
          (:then_1
            (Utilities|FlowControl|Gate false) ; enters at Open
          )
          (:then_2
            (Utilities|FlowControl|Gate false) ; enters at Open
          )
          (:then_3
            (Utilities|FlowControl|Gate false) ; enters at Open
          )))))
  (:Completed
    (bind _output_get (Variables|Default|SetGetIA_ThrottleDown false))))

(event Input|EnhancedActionEvents|EnhancedInputActionIA_PitchUp
  (params (ActionValue :type Boolean) (ElapsedSeconds :type Float%20%28double-precision%29) (TriggeredSeconds :type Float%20%28double-precision%29) (InputAction :type Input%20Action%20Object%20Reference :default "/FPVAcroDrones/Input/Actions/IA_PitchUp.IA_PitchUp"))
  (bind _playercontroller (Variables|Default|GetPlayerController))
  (:Triggered
    ;[0.15 0.15 0.15 0.5] Keyboard
    ;;[0.15 0.15 0.15 0.5] Keyboard Pitch
    (bind _output_get (Variables|Default|SetGetIA_PitchUp true))
    ;;[0.15 0.15 0.15 0.5] Block Keyboard Input (note that Steam also adds arrow key events to the gamepad)
    (Utilities|FlowControl|Gate false :!label _label
      (:Exit
        (Utilities|IsValid _playercontroller
          (:Is%20Valid
            (Class|EnhancedInputSubsystemInterface|InjectInputVectorforAction (PlayerController|LocalPlayerSubsystems|GetEnhancedInputLocalPlayerSubsystem _playercontroller) "/FPVAcroDrones/Input/Actions/IA_PitchInjected.IA_PitchInjected" (Math|Vector|MakeVector (+ (select _output_get -1.0 0.0) (select (stale Input|EnhancedActionEvents|EnhancedInputActionIA_PitchDown _output_get) 1.0 0.0)) 0.0 0.0)))))))
  (:Completed
    (Variables|Default|SetGetIA_PitchUp false)
    (goto _label)))

(event Input|EnhancedActionEvents|EnhancedInputActionIA_PitchDown
  (params (ActionValue :type Boolean) (ElapsedSeconds :type Float%20%28double-precision%29) (TriggeredSeconds :type Float%20%28double-precision%29) (InputAction :type Input%20Action%20Object%20Reference :default "/FPVAcroDrones/Input/Actions/IA_PitchDown.IA_PitchDown"))
  (bind _playercontroller (Variables|Default|GetPlayerController))
  (:Triggered
    ;[0.15 0.15 0.15 0.5] Keyboard
    ;;[0.15 0.15 0.15 0.5] Keyboard Pitch
    (Variables|Default|SetGetIA_PitchDown true)
    ;;[0.15 0.15 0.15 0.5] Block Keyboard Input (note that Steam also adds arrow key events to the gamepad)
    (Utilities|FlowControl|Gate false :!label _label
      (:Exit
        (Utilities|IsValid _playercontroller
          (:Is%20Valid
            (Class|EnhancedInputSubsystemInterface|InjectInputVectorforAction (PlayerController|LocalPlayerSubsystems|GetEnhancedInputLocalPlayerSubsystem _playercontroller) "/FPVAcroDrones/Input/Actions/IA_PitchInjected.IA_PitchInjected" (Math|Vector|MakeVector (+ (select (stale Input|EnhancedActionEvents|EnhancedInputActionIA_PitchUp _output_get) -1.0 0.0) (select (stale _output_get) 1.0 0.0)) 0.0 0.0)))))))
  (:Completed
    (bind _output_get (Variables|Default|SetGetIA_PitchDown false))
    (goto _label)))

(event Input|EnhancedActionEvents|EnhancedInputActionIA_RollLeft
  (params (ActionValue :type Boolean) (ElapsedSeconds :type Float%20%28double-precision%29) (TriggeredSeconds :type Float%20%28double-precision%29) (InputAction :type Input%20Action%20Object%20Reference :default "/FPVAcroDrones/Input/Actions/IA_RollLeft.IA_RollLeft"))
  (bind _playercontroller (Variables|Default|GetPlayerController))
  (:Triggered
    ;[0.15 0.15 0.15 0.5] Keyboard
    ;;[0.15 0.15 0.15 0.5] Keyboard Roll
    (bind _output_get (Variables|Default|SetGetIA_RollLeft true))
    ;;[0.15 0.15 0.15 0.5] Block Keyboard Input (note that Steam also adds arrow key events to the gamepad)
    (Utilities|FlowControl|Gate false :!label _label
      (:Exit
        (Utilities|IsValid _playercontroller
          (:Is%20Valid
            (Class|EnhancedInputSubsystemInterface|InjectInputVectorforAction (PlayerController|LocalPlayerSubsystems|GetEnhancedInputLocalPlayerSubsystem _playercontroller) "/FPVAcroDrones/Input/Actions/IA_RollInjected.IA_RollInjected" (Math|Vector|MakeVector (+ (select _output_get -1.0 0.0) (select (stale Input|EnhancedActionEvents|EnhancedInputActionIA_RollRight _output_get) 1.0 0.0)) 0.0 0.0)))))))
  (:Completed
    (Variables|Default|SetGetIA_RollLeft false)
    (goto _label)))

(event Input|EnhancedActionEvents|EnhancedInputActionIA_RollRight
  (params (ActionValue :type Boolean) (ElapsedSeconds :type Float%20%28double-precision%29) (TriggeredSeconds :type Float%20%28double-precision%29) (InputAction :type Input%20Action%20Object%20Reference :default "/FPVAcroDrones/Input/Actions/IA_RollRight.IA_RollRight"))
  (bind _playercontroller (Variables|Default|GetPlayerController))
  (:Triggered
    ;[0.15 0.15 0.15 0.5] Keyboard
    ;;[0.15 0.15 0.15 0.5] Keyboard Roll
    (Variables|Default|SetGetIA_RollRight true)
    ;;[0.15 0.15 0.15 0.5] Block Keyboard Input (note that Steam also adds arrow key events to the gamepad)
    (Utilities|FlowControl|Gate false :!label _label
      (:Exit
        (Utilities|IsValid _playercontroller
          (:Is%20Valid
            (Class|EnhancedInputSubsystemInterface|InjectInputVectorforAction (PlayerController|LocalPlayerSubsystems|GetEnhancedInputLocalPlayerSubsystem _playercontroller) "/FPVAcroDrones/Input/Actions/IA_RollInjected.IA_RollInjected" (Math|Vector|MakeVector (+ (select (stale Input|EnhancedActionEvents|EnhancedInputActionIA_RollLeft _output_get) -1.0 0.0) (select (stale _output_get) 1.0 0.0)) 0.0 0.0)))))))
  (:Completed
    (bind _output_get (Variables|Default|SetGetIA_RollRight false))
    (goto _label)))

(event Input|EnhancedActionEvents|EnhancedInputActionIA_YawInjected
  (params (ActionValue :type Float%20%28double-precision%29) (ElapsedSeconds :type Float%20%28double-precision%29) (TriggeredSeconds :type Float%20%28double-precision%29) (InputAction :type Input%20Action%20Object%20Reference :default "/FPVAcroDrones/Input/Actions/IA_YawInjected.IA_YawInjected"))
  (bind _playercontroller (Variables|Default|GetPlayerController))
  ;[0.15 0.15 0.15 0.5] Pass to the Input Actions with the Response Curves
  (Utilities|IsValid _playercontroller
    (:Is%20Valid
      (Class|EnhancedInputSubsystemInterface|InjectInputVectorforAction (PlayerController|LocalPlayerSubsystems|GetEnhancedInputLocalPlayerSubsystem _playercontroller) "/FPVAcroDrones/Input/Actions/IA_YawFPVAcroDrone.IA_YawFPVAcroDrone" (Math|Vector|MakeVector ActionValue 0.0 0.0)))))

(event Input|EnhancedActionEvents|EnhancedInputActionIA_RollInjected
  (params (ActionValue :type Float%20%28double-precision%29) (ElapsedSeconds :type Float%20%28double-precision%29) (TriggeredSeconds :type Float%20%28double-precision%29) (InputAction :type Input%20Action%20Object%20Reference :default "/FPVAcroDrones/Input/Actions/IA_RollInjected.IA_RollInjected"))
  (bind _playercontroller (Variables|Default|GetPlayerController))
  ;[0.15 0.15 0.15 0.5] Pass to the Input Actions with the Response Curves
  (Utilities|IsValid _playercontroller
    (:Is%20Valid
      (Class|EnhancedInputSubsystemInterface|InjectInputVectorforAction (PlayerController|LocalPlayerSubsystems|GetEnhancedInputLocalPlayerSubsystem _playercontroller) "/FPVAcroDrones/Input/Actions/IA_RollFPVAcroDrone.IA_RollFPVAcroDrone" (Math|Vector|MakeVector ActionValue 0.0 0.0)))))

(event Input|EnhancedActionEvents|EnhancedInputActionIA_Throttle
  (params (ActionValue :type Float%20%28double-precision%29) (ElapsedSeconds :type Float%20%28double-precision%29) (TriggeredSeconds :type Float%20%28double-precision%29) (InputAction :type Input%20Action%20Object%20Reference :default "/FPVAcroDrones/Input/Actions/IA_Throttle.IA_Throttle"))
  (bind _playercontroller (Variables|Default|GetPlayerController))
  (bind _returnvalue (PlayerController|LocalPlayerSubsystems|GetEnhancedInputLocalPlayerSubsystem _playercontroller))
  ;[0.15 0.15 0.15 0.5] Gamepad
  (Class|EnhancedInputSubsystemInterface|InjectInputVectorforAction (PlayerController|LocalPlayerSubsystems|GetEnhancedInputLocalPlayerSubsystem (Variables|Default|GetPlayerController)) "/FPVAcroDrones/Input/Actions/IA_ThrottleInjected.IA_ThrottleInjected" (Math|Vector|MakeVector ActionValue 0.0 0.0))
  ;[0.15 0.15 0.15 0.5] Keyboard
  ;;[0.15 0.15 0.15 0.5] Block Keyboard Input (note that Steam also adds arrow key events to the gamepad)
  (Variables|Default|SetThrottleTrim 0.0)
  (Utilities|FlowControl|Sequence
    (:then_0
      (Utilities|FlowControl|Gate false) ; enters at Close
    )
    (:then_1
      (Utilities|FlowControl|Gate false) ; enters at Close
    )
    (:then_2
      (Utilities|FlowControl|Gate false) ; enters at Close
    )
    (:then_3
      (Utilities|FlowControl|Gate false) ; enters at Close
    )))

(event Input|EnhancedActionEvents|EnhancedInputActionIA_Yaw
  (params (ActionValue :type Float%20%28double-precision%29) (ElapsedSeconds :type Float%20%28double-precision%29) (TriggeredSeconds :type Float%20%28double-precision%29) (InputAction :type Input%20Action%20Object%20Reference :default "/FPVAcroDrones/Input/Actions/IA_Yaw.IA_Yaw"))
  (bind _playercontroller (Variables|Default|GetPlayerController))
  (bind _returnvalue (PlayerController|LocalPlayerSubsystems|GetEnhancedInputLocalPlayerSubsystem _playercontroller))
  ;[0.15 0.15 0.15 0.5] Gamepad
  (Class|EnhancedInputSubsystemInterface|InjectInputVectorforAction (PlayerController|LocalPlayerSubsystems|GetEnhancedInputLocalPlayerSubsystem (Variables|Default|GetPlayerController)) "/FPVAcroDrones/Input/Actions/IA_YawInjected.IA_YawInjected" (Math|Vector|MakeVector ActionValue 0.0 0.0))
  ;[0.15 0.15 0.15 0.5] Keyboard
  ;;[0.15 0.15 0.15 0.5] Block Keyboard Input (note that Steam also adds arrow key events to the gamepad)
  (Variables|Default|SetThrottleTrim 0.0)
  (Utilities|FlowControl|Sequence
    (:then_0
      (Utilities|FlowControl|Gate false) ; enters at Close
    )
    (:then_1
      (Utilities|FlowControl|Gate false) ; enters at Close
    )
    (:then_2
      (Utilities|FlowControl|Gate false) ; enters at Close
    )
    (:then_3
      (Utilities|FlowControl|Gate false) ; enters at Close
    )))

(event Input|EnhancedActionEvents|EnhancedInputActionIA_Pitch
  (params (ActionValue :type Float%20%28double-precision%29) (ElapsedSeconds :type Float%20%28double-precision%29) (TriggeredSeconds :type Float%20%28double-precision%29) (InputAction :type Input%20Action%20Object%20Reference :default "/FPVAcroDrones/Input/Actions/IA_Pitch.IA_Pitch"))
  (bind _playercontroller (Variables|Default|GetPlayerController))
  (bind _returnvalue (PlayerController|LocalPlayerSubsystems|GetEnhancedInputLocalPlayerSubsystem _playercontroller))
  ;[0.15 0.15 0.15 0.5] Gamepad
  (Class|EnhancedInputSubsystemInterface|InjectInputVectorforAction (PlayerController|LocalPlayerSubsystems|GetEnhancedInputLocalPlayerSubsystem (Variables|Default|GetPlayerController)) "/FPVAcroDrones/Input/Actions/IA_PitchInjected.IA_PitchInjected" (Math|Vector|MakeVector ActionValue 0.0 0.0))
  ;[0.15 0.15 0.15 0.5] Keyboard
  ;;[0.15 0.15 0.15 0.5] Block Keyboard Input (note that Steam also adds arrow key events to the gamepad)
  (Variables|Default|SetThrottleTrim 0.0)
  (Utilities|FlowControl|Sequence
    (:then_0
      (Utilities|FlowControl|Gate false) ; enters at Close
    )
    (:then_1
      (Utilities|FlowControl|Gate false) ; enters at Close
    )
    (:then_2
      (Utilities|FlowControl|Gate false) ; enters at Close
    )
    (:then_3
      (Utilities|FlowControl|Gate false) ; enters at Close
    )))

(event Input|EnhancedActionEvents|EnhancedInputActionIA_Roll
  (params (ActionValue :type Float%20%28double-precision%29) (ElapsedSeconds :type Float%20%28double-precision%29) (TriggeredSeconds :type Float%20%28double-precision%29) (InputAction :type Input%20Action%20Object%20Reference :default "/FPVAcroDrones/Input/Actions/IA_Roll.IA_Roll"))
  (bind _playercontroller (Variables|Default|GetPlayerController))
  (bind _returnvalue (PlayerController|LocalPlayerSubsystems|GetEnhancedInputLocalPlayerSubsystem _playercontroller))
  ;[0.15 0.15 0.15 0.5] Gamepad
  (Class|EnhancedInputSubsystemInterface|InjectInputVectorforAction (PlayerController|LocalPlayerSubsystems|GetEnhancedInputLocalPlayerSubsystem (Variables|Default|GetPlayerController)) "/FPVAcroDrones/Input/Actions/IA_RollInjected.IA_RollInjected" (Math|Vector|MakeVector ActionValue 0.0 0.0))
  ;[0.15 0.15 0.15 0.5] Keyboard
  ;;[0.15 0.15 0.15 0.5] Block Keyboard Input (note that Steam also adds arrow key events to the gamepad)
  (Variables|Default|SetThrottleTrim 0.0)
  (Utilities|FlowControl|Sequence
    (:then_0
      (Utilities|FlowControl|Gate false) ; enters at Close
    )
    (:then_1
      (Utilities|FlowControl|Gate false) ; enters at Close
    )
    (:then_2
      (Utilities|FlowControl|Gate false) ; enters at Close
    )
    (:then_3
      (Utilities|FlowControl|Gate false) ; enters at Close
    )))

(event Input|EnhancedActionEvents|EnhancedInputActionIA_ThrottleInjected
  (params (ActionValue :type Float%20%28double-precision%29) (ElapsedSeconds :type Float%20%28double-precision%29) (TriggeredSeconds :type Float%20%28double-precision%29) (InputAction :type Input%20Action%20Object%20Reference :default "/FPVAcroDrones/Input/Actions/IA_ThrottleInjected.IA_ThrottleInjected"))
  (bind _playercontroller (Variables|Default|GetPlayerController))
  ;[0.15 0.15 0.15 0.5] Pass to the Input Actions with the Response Curves
  (Utilities|IsValid _playercontroller
    (:Is%20Valid
      (Class|EnhancedInputSubsystemInterface|InjectInputVectorforAction (PlayerController|LocalPlayerSubsystems|GetEnhancedInputLocalPlayerSubsystem _playercontroller) "/FPVAcroDrones/Input/Actions/IA_ThrottleFPVAcroDrone.IA_ThrottleFPVAcroDrone" (Math|Vector|MakeVector ActionValue 0.0 0.0)))))

(event Input|EnhancedActionEvents|EnhancedInputActionIA_YawLeft
  (params (ActionValue :type Boolean) (ElapsedSeconds :type Float%20%28double-precision%29) (TriggeredSeconds :type Float%20%28double-precision%29) (InputAction :type Input%20Action%20Object%20Reference :default "/FPVAcroDrones/Input/Actions/IA_YawLeft.IA_YawLeft"))
  (bind _playercontroller (Variables|Default|GetPlayerController))
  (:Triggered
    ;[0.15 0.15 0.15 0.5] Keyboard
    ;;[0.15 0.15 0.15 0.5] Keyboard Yaw
    (bind _output_get (Variables|Default|SetGetIA_YawLeft true))
    ;;[0.15 0.15 0.15 0.5] Block Keyboard Input (note that Steam also adds arrow key events to the gamepad)
    (Utilities|FlowControl|Gate false :!label _label
      (:Exit
        (Utilities|IsValid _playercontroller
          (:Is%20Valid
            (Class|EnhancedInputSubsystemInterface|InjectInputVectorforAction (PlayerController|LocalPlayerSubsystems|GetEnhancedInputLocalPlayerSubsystem _playercontroller) "/FPVAcroDrones/Input/Actions/IA_YawInjected.IA_YawInjected" (Math|Vector|MakeVector (+ (select _output_get -1.0 0.0) (select (stale Input|EnhancedActionEvents|EnhancedInputActionIA_YawRight _output_get) 1.0 0.0)) 0.0 0.0)))))))
  (:Completed
    (Variables|Default|SetGetIA_YawLeft false)
    (goto _label)))

(event Input|EnhancedActionEvents|EnhancedInputActionIA_PitchInjected
  (params (ActionValue :type Float%20%28double-precision%29) (ElapsedSeconds :type Float%20%28double-precision%29) (TriggeredSeconds :type Float%20%28double-precision%29) (InputAction :type Input%20Action%20Object%20Reference :default "/FPVAcroDrones/Input/Actions/IA_PitchInjected.IA_PitchInjected"))
  (bind _playercontroller (Variables|Default|GetPlayerController))
  ;[0.15 0.15 0.15 0.5] Pass to the Input Actions with the Response Curves
  (Utilities|IsValid _playercontroller
    (:Is%20Valid
      (Class|EnhancedInputSubsystemInterface|InjectInputVectorforAction (PlayerController|LocalPlayerSubsystems|GetEnhancedInputLocalPlayerSubsystem _playercontroller) "/FPVAcroDrones/Input/Actions/IA_PitchFPVAcroDrone.IA_PitchFPVAcroDrone" (Math|Vector|MakeVector ActionValue 0.0 0.0)))))

(event Input|EnhancedActionEvents|EnhancedInputActionIA_YawRight
  (params (ActionValue :type Boolean) (ElapsedSeconds :type Float%20%28double-precision%29) (TriggeredSeconds :type Float%20%28double-precision%29) (InputAction :type Input%20Action%20Object%20Reference :default "/FPVAcroDrones/Input/Actions/IA_YawRight.IA_YawRight"))
  (bind _playercontroller (Variables|Default|GetPlayerController))
  (:Triggered
    ;[0.15 0.15 0.15 0.5] Keyboard
    ;;[0.15 0.15 0.15 0.5] Keyboard Yaw
    (Variables|Default|SetGetIA_YawRight true)
    ;;[0.15 0.15 0.15 0.5] Block Keyboard Input (note that Steam also adds arrow key events to the gamepad)
    (Utilities|FlowControl|Gate false :!label _label
      (:Exit
        (Utilities|IsValid _playercontroller
          (:Is%20Valid
            (Class|EnhancedInputSubsystemInterface|InjectInputVectorforAction (PlayerController|LocalPlayerSubsystems|GetEnhancedInputLocalPlayerSubsystem _playercontroller) "/FPVAcroDrones/Input/Actions/IA_YawInjected.IA_YawInjected" (Math|Vector|MakeVector (+ (select (stale Input|EnhancedActionEvents|EnhancedInputActionIA_YawLeft _output_get) -1.0 0.0) (select (stale _output_get) 1.0 0.0)) 0.0 0.0)))))))
  (:Completed
    (bind _output_get (Variables|Default|SetGetIA_YawRight false))
    (goto _label)))

(event EventBeginPlay
  ;[0.15 0.15 0.15 0.5] Get Player Controller from the Owning Actor
  (bind _asequip_fpvacro_drone_rc (Utilities|Casting|CastToEquip_FPVAcroDroneRC (Components|GetOwner))
    (:then
      (EventDispatchers|BindEventtoPlayerControllerSet _asequip_fpvacro_drone_rc (delegate Custom|Event%20Was%20Equipped)))
    (:CastFailed
      ;;[1 0.15 0.15 0.5] Blueprint Assert
      (Class|BlueprintLoggingLibrary|LogFatal "Can't get RC. Will not control the drone."))))

(event EventTick
  (params (DeltaSeconds :type Float%20%28single-precision%29))
  (bind _playercontroller (Variables|Default|GetPlayerController))
  ;[0.15 0.15 0.15 0.5] Keyboard
  ;;[0.15 0.15 0.15 0.5] Keyboard Throttle
  (bind _output_get (Variables|Default|SetThrottleTrim (Math|Float|Clamp(Float) (+ (* 2.0 DeltaSeconds (+ (select (stale Input|EnhancedActionEvents|EnhancedInputActionIA_ThrottleUp _output_get) 1.0 0.0) (select (stale Input|EnhancedActionEvents|EnhancedInputActionIA_ThrottleDown _output_get) -1.0 0.0))) (Variables|Default|GetThrottleTrim)))))
  ;;[0.15 0.15 0.15 0.5] Block Keyboard Input (note that Steam also adds arrow key events to the gamepad)
  (Utilities|FlowControl|Gate false
    (:Exit
      (Utilities|IsValid _playercontroller
        (:Is%20Valid
          (Class|EnhancedInputSubsystemInterface|InjectInputVectorforAction (PlayerController|LocalPlayerSubsystems|GetEnhancedInputLocalPlayerSubsystem _playercontroller) "/FPVAcroDrones/Input/Actions/IA_ThrottleInjected.IA_ThrottleInjected" (Math|Vector|MakeVector _output_get 0.0 0.0)))))))