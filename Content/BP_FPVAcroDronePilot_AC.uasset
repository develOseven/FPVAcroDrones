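; Pilot component for the FPV acro drone mod's player character, tracking goggles-equipped state and handling custom body meshes.
; Five seconds after BeginPlay, it copies first- and third-person mesh visibility onto custom skeletal meshes, hides the originals and fires CameraChanged.
; A temporary debug input toggles first/third-person camera, debounced by a timer-reset DoOnce, and reruns the mesh swap.
; Several disconnected debug logging and teleport snippets never run.
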(event Custom|CamChange
  (bind _returnvalue (Utilities|Enum|LiteralenumECameraMode "ECM_FirstPerson"))
  ;[0.15 0.15 0.15 0.5] TODO: why Pressed double-fires?
  (Utilities|FlowControl|DoOnce false) ; enters at Reset
)

(event Custom|Event%20GooglesEquippedChanged
  (params (Equipped :type Boolean))
  ;[0.15 0.15 0.15 0.5] Googles State and Notification
  (Variables|Default|SetGooglesEquipped Equipped))

(event Custom|Poll)

(event Custom|CustomEvent
  (params (Pawn :type Pawn%20Object%20Reference) (Controller :type Controller%20Object%20Reference))
  (Class|BlueprintLoggingLibrary|LogDisplay (Utilities|String|Append "Controller: " (Utilities|GetDisplayName Controller) (Utilities|GetDisplayName Pawn))))

(event Custom|EventInitCustomMeshesVisibility
  ;[0.15 0.15 0.15 0.5] TODO: track palyer mesh visibility instead of just once after begin
  ;[0.15 0.15 0.15 0.5] TODO: rm Debug 3P Camera
  ;;[0.15 0.15 0.15 0.5] Adapt visibility of the custom meshes
  (bind _asfgcharacter_player (Utilities|Casting|CastToFGCharacterPlayer (Components|GetOwner))
    (:then
      (Utilities|FlowControl|Sequence
        (:then_0
          (if (Rendering|IsVisible (Class|FGCharacterPlayer|Get3PMesh _asfgcharacter_player))
            (Variables|/Script/Engine.SkinnedMeshComponent|SetVisibilityBasedAnimTickOption (Class|FGCharacterPlayer|Get3PMesh _asfgcharacter_player) "AlwaysTickPoseAndRefreshBones")))
        (:then_1
          (Rendering|SetVisibility (Variables|Default|GetcustomSkeletalMesh3P) (Rendering|IsVisible (Class|FGCharacterPlayer|Get3PMesh _asfgcharacter_player)) false)
          (Utilities|FlowControl|Sequence
            (:then_0
              (Rendering|SetVisibility (Variables|Default|GetcustomSkeletalMesh1P) (Rendering|IsVisible (Class|FGCharacterPlayer|GetMesh1P _asfgcharacter_player)) false)
              (Rendering|SetVisibility (Class|FGCharacterPlayer|Get3PMesh _asfgcharacter_player) false false)
              (Rendering|SetVisibility (Class|FGCharacterPlayer|GetMesh1P _asfgcharacter_player) false false)
              (Class|BlueprintLoggingLibrary|LogDisplay (Utilities|String|Append "1P Visible: " (Utilities|String|ToString(Boolean) (Rendering|IsVisible (Class|FGCharacterPlayer|GetMesh1P _asfgcharacter_player)))))
              (Class|BlueprintLoggingLibrary|LogDisplay (Utilities|String|Append "3P Visible: " (Utilities|String|ToString(Boolean) (Rendering|IsVisible (Class|FGCharacterPlayer|Get3PMesh _asfgcharacter_player)))))
              (Default|CallCameraChanged))
            (:then_1
              (if (Rendering|IsVisible (Class|FGCharacterPlayer|GetMesh1P _asfgcharacter_player))
                (Variables|/Script/Engine.SkinnedMeshComponent|SetVisibilityBasedAnimTickOption (Class|FGCharacterPlayer|GetMesh1P _asfgcharacter_player) "AlwaysTickPoseAndRefreshBones")))))))
    (:CastFailed
      ;;;[1 0.15 0.15 0.5] Blueprint Assert
      (Class|BlueprintLoggingLibrary|LogFatal "Can't get Character Player. Will not get mesh debug info."))))

(event Input|EnhancedActionEvents|EnhancedInputActionIA_ToggleCameraMode
  (params (ActionValue :type Boolean) (ElapsedSeconds :type Float%20%28double-precision%29) (TriggeredSeconds :type Float%20%28double-precision%29) (InputAction :type Input%20Action%20Object%20Reference :default "/FPVAcroDrones/Input/Actions/IA_ToggleCameraMode.IA_ToggleCameraMode"))
  (bind _returnvalue (Utilities|Enum|LiteralenumECameraMode "ECM_FirstPerson"))
  ;[0.15 0.15 0.15 0.5] TODO: why Pressed double-fires?
  (Utilities|FlowControl|DoOnce false
    (:Completed
      (Utilities|Time|SetTimerbyEvent (delegate Custom|CamChange) 0.2)
      ;[0.15 0.15 0.15 0.5] TODO: rm Debug 3P Camera
      (Class|BlueprintLoggingLibrary|LogDisplay "Cam toggle")
      (bind _asfgcharacter_player (Utilities|Casting|CastToFGCharacterPlayer (Components|GetOwner))
        (:then
          (Class|FGCharacterPlayer|SetCameraMode _asfgcharacter_player (select (Utilities|Enum|NotEqual(Enum) _returnvalue (Class|FGCharacterPlayer|GetCameraMode _asfgcharacter_player)) _returnvalue (Utilities|Enum|LiteralenumECameraMode "ECM_ThirdPerson")))
          ;;[0.15 0.15 0.15 0.5] Adapt visibility of the custom meshes
          (bind _asfgcharacter_player_2 (Utilities|Casting|CastToFGCharacterPlayer (Components|GetOwner))
            (:then
              (Utilities|FlowControl|Sequence
                (:then_0
                  (if (Rendering|IsVisible (Class|FGCharacterPlayer|Get3PMesh _asfgcharacter_player_2))
                    (Variables|/Script/Engine.SkinnedMeshComponent|SetVisibilityBasedAnimTickOption (Class|FGCharacterPlayer|Get3PMesh _asfgcharacter_player_2) "AlwaysTickPoseAndRefreshBones")))
                (:then_1
                  (Rendering|SetVisibility (Variables|Default|GetcustomSkeletalMesh3P) (Rendering|IsVisible (Class|FGCharacterPlayer|Get3PMesh _asfgcharacter_player_2)) false)
                  (Utilities|FlowControl|Sequence
                    (:then_0
                      (Rendering|SetVisibility (Variables|Default|GetcustomSkeletalMesh1P) (Rendering|IsVisible (Class|FGCharacterPlayer|GetMesh1P _asfgcharacter_player_2)) false)
                      (Rendering|SetVisibility (Class|FGCharacterPlayer|Get3PMesh _asfgcharacter_player_2) false false)
                      (Rendering|SetVisibility (Class|FGCharacterPlayer|GetMesh1P _asfgcharacter_player_2) false false)
                      (Class|BlueprintLoggingLibrary|LogDisplay (Utilities|String|Append "1P Visible: " (Utilities|String|ToString(Boolean) (Rendering|IsVisible (Class|FGCharacterPlayer|GetMesh1P _asfgcharacter_player_2)))))
                      (Class|BlueprintLoggingLibrary|LogDisplay (Utilities|String|Append "3P Visible: " (Utilities|String|ToString(Boolean) (Rendering|IsVisible (Class|FGCharacterPlayer|Get3PMesh _asfgcharacter_player_2)))))
                      (Default|CallCameraChanged))
                    (:then_1
                      (if (Rendering|IsVisible (Class|FGCharacterPlayer|GetMesh1P _asfgcharacter_player_2))
                        (Variables|/Script/Engine.SkinnedMeshComponent|SetVisibilityBasedAnimTickOption (Class|FGCharacterPlayer|GetMesh1P _asfgcharacter_player_2) "AlwaysTickPoseAndRefreshBones")))))))
            (:CastFailed
              ;;;[1 0.15 0.15 0.5] Blueprint Assert
              (Class|BlueprintLoggingLibrary|LogFatal "Can't get Character Player. Will not get mesh debug info."))))
        (:CastFailed
          ;;[1 0.15 0.15 0.5] Blueprint Assert
          (Class|BlueprintLoggingLibrary|LogFatal "Can't get Character Player Controller. Will not switch debug camera."))))))

(event EventBeginPlay
  (bind _returnvalue (Components|GetOwner))
  (bind _returnvalue_2 (Game|GetInstigatorController _returnvalue))
  (Utilities|FlowControl|Sequence
    (:then_0
      (Class|BlueprintLoggingLibrary|LogDisplay "Pilot begun play"))
    (:then_1
      ;[0.15 0.15 0.15 0.5] Googles State and Notification
      (EventDispatchers|BindEventtoGooglesEquippedChanged (delegate Custom|Event%20GooglesEquippedChanged)))
    (:then_2
      ;[0.15 0.15 0.15 0.5] TODO: track palyer mesh visibility instead of just once after begin
      (Utilities|Time|SetTimerbyEvent (delegate Custom|EventInitCustomMeshesVisibility) 5.0))
    (:then_3
      ;[0.15 0.15 0.15 0.5] TODO: rm debug camera input
      (Utilities|IsValid _returnvalue_2
        (:Is%20Valid
          (bind _asplayer_controller (Utilities|Casting|CastToPlayerController _returnvalue_2)
            (:then
              (Input|AddMappingContext (PlayerController|LocalPlayerSubsystems|GetEnhancedInputLocalPlayerSubsystem _asplayer_controller) "/FPVAcroDrones/Input/IMC_Camera.IMC_Camera" 0 "(bIgnoreAllPressedKeysUntilRelease=1,bForceImmediately=0,bNotifyUserSettings=False)"))
            (:CastFailed
              ;;[1 0.15 0.15 0.5] Blueprint Assert
              (Class|BlueprintLoggingLibrary|LogFatal "Can't get Character Player Controller. Will not switch debug camera."))))))))